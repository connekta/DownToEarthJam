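; NavigationPoint is a waypoint actor that passes zombies along a chain of points.
; When an actor of exactly the Zombie_Base class begins overlapping it, it prints a debug string and calls MoveToNextPoint on the zombie with its linked NextPoint.
; The construction script rotates an Arrow component to face NextPoint, showing the link direction, with no validity check on that reference.
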(event `self.ReceiveActorBeginOverlap`
  (params (OtherActor :type "Actor Object Reference"))
  (if (== (`GameplayStatics.GetObjectClass` OtherActor) "/Game/Blueprints/Zombie_Base.Zombie_Base_C")
    (`KismetSystemLibrary.PrintString` "Zombie Entered Zone")
    (bind _aszombie_base (cast `/Game/Blueprints/Zombie_Base` OtherActor))
    (`/Game/Blueprints/Zombie_Base.MoveToNextPoint` _aszombie_base (`self.NextPoint`))))

(fn `UserConstructionScript`
  (`SceneComponent.K2_SetWorldRotation` (`self.Arrow`) (`KismetMathLibrary.FindLookAtRotation` (`self.K2_GetActorLocation`) (`self.K2_GetActorLocation` (`self.NextPoint`))) false false))