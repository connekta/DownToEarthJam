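; Base shop item actor that shows its cost and description and sells itself to the interacting player.
; BeginPlay fills both texts and starts a timeline that lifts the mesh for a bobbing motion.
; Tick rotates the whole actor twice for text billboarding, so the second, description-based rotation overrides the first.
; Interaction deducts affordable costs from player Currency, calls the empty BoughtThisItem hook and destroys the item, otherwise printing a message.
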(event `self.ReceiveBeginPlay`
  (bind _startloc (`self.StartLoc`))
  ;[1 1 1] Set Cost Text
  (`TextRenderComponent.K2_SetText` (`self.CostText`) (`KismetTextLibrary.Conv_StringToText` (`KismetStringLibrary.Concat_StrStr` "Cost: " (`KismetStringLibrary.Conv_IntToString` (`self.Cost`)))))
  (`TextRenderComponent.K2_SetText` (`self.DescriptionText`) (`KismetTextLibrary.Conv_StringToText` (`self.ItemDescription`)))
  (set `self.StartLoc` (`SceneComponent.K2_GetComponentLocation` (`self.InteractableMesh`)))
  (`|ExecutionSequence`
    (:`then_0`
      (bind (_direction _newtrack_0) (`Timeline|UpDown` :!via `PlayFromStart`)
        (:`Update`
          (`SceneComponent.K2_SetWorldLocation` (`self.InteractableMesh`) (`KismetMathLibrary.VLerp` _startloc (+ _startloc (0.0 0.0 10.0)) _newtrack_0) false false))))))

(event `self.ReceiveTick`
  (params (DeltaSeconds :type "Float (single-precision)"))
  ;[1 1 1] Billboard Text
  (`self.K2_SetActorRotation` (`KismetMathLibrary.FindLookAtRotation` (`SceneComponent.K2_GetComponentLocation` (`self.CostText`)) (`self.K2_GetActorLocation` (`GameplayStatics.GetPlayerCameraManager` 0))))
  (`self.K2_SetActorRotation` (`KismetMathLibrary.MakeRotFromX` (- (`SceneComponent.K2_GetComponentLocation` (`self.DescriptionText`)) (`self.K2_GetActorLocation` (`GameplayStatics.GetPlayerCameraManager` 0))))))

(event `/Game/Blueprints/InteractableInterface.InteractedFunction`
  (params (PlayerInteracted :type "/Game/Blueprints/ThirdPersonCharacter Object Reference"))
  (bind _currency (`/Game/Blueprints/ThirdPersonCharacter.Currency` PlayerInteracted))
  (bind _cost (`self.Cost`))
  (set `self.InteractedPlayer` PlayerInteracted)
  (if (>= _currency _cost)
    (set `/Game/Blueprints/ThirdPersonCharacter.Currency` (- _currency _cost) PlayerInteracted)
    (`/Game/Blueprints/ThirdPersonCharacter.UpdateCurrencyFromRemote` PlayerInteracted)
    (`self.BoughtThisItem`)
    (`self.K2_DestroyActor`)
    (else
      (`KismetSystemLibrary.PrintString` "Cant afford item"))))

(fn `BoughtThisItem`)

(fn `UserConstructionScript`)