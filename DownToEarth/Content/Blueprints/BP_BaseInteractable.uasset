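; BP_BaseInteractable is a base Blueprint for objects the player character can interact with.
; While active, its InteractableArea registers it with an overlapping ThirdPersonCharacter through RegisterInteractableMessage and unregisters it when the overlap ends.
; SetHighlight toggles custom depth rendering on the static mesh and, when valid, the skeletal mesh.
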(event `self.InteractableArea.OnComponentBeginOverlap`
  (params (OverlappedComponent :type "PrimitiveComponent Object Reference") (OtherActor :type "Actor Object Reference") (OtherComp :type "PrimitiveComponent Object Reference") (OtherBodyIndex :type Integer) (bFromSweep :type Boolean) (SweepResult :type "HitResult Structure (by ref)"))
  (if (`self.IsActive?`)
    (bind _asthird_person_character (cast `/Game/Blueprints/ThirdPersonCharacter` OtherActor))
    (message `/Game/Blueprints/InteractableInterface.RegisterInteractable` _asthird_person_character self)))

(event `self.InteractableArea.OnComponentEndOverlap`
  (params (OverlappedComponent :type "PrimitiveComponent Object Reference") (OtherActor :type "Actor Object Reference") (OtherComp :type "PrimitiveComponent Object Reference") (OtherBodyIndex :type Integer))
  (if (`self.IsActive?`)
    (bind _asthird_person_character (cast `/Game/Blueprints/ThirdPersonCharacter` OtherActor))
    (message `/Game/Blueprints/InteractableInterface.UnregisterInteractable` _asthird_person_character self)))

(fn `SetHighlight`
  (params (`Highlight?` :type Boolean))
  (bind _interactableskelmesh (`self.InteractableSkelMesh`))
  (`PrimitiveComponent.SetRenderCustomDepth` (`self.InteractableMesh`) `Highlight?`)
  (if (`KismetSystemLibrary.IsValid` _interactableskelmesh)
    (`PrimitiveComponent.SetRenderCustomDepth` _interactableskelmesh `Highlight?`)))

(fn `UserConstructionScript`)