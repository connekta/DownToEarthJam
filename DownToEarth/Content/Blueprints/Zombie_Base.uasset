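; Base zombie character that chases and melees players, then becomes a corpse they can carry.
; It picks the nearest player at BeginPlay, re-issues AIMoveTo once navigation is enabled, and attacks at close range.
; Non-lethal hits turn a random body part physical, while death ragdolls it and launches a WeddingRing drop.
; Corpses highlight via custom depth and swap to the ZombieLOCKED mesh while carried; nav-point wandering is unwired.
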(event `self.ZombieCorpseRadius.OnComponentBeginOverlap`
  (params (OverlappedComponent :type "PrimitiveComponent Object Reference") (OtherActor :type "Actor Object Reference") (OtherComp :type "PrimitiveComponent Object Reference") (OtherBodyIndex :type Integer) (bFromSweep :type Boolean) (SweepResult :type "HitResult Structure (by ref)"))
  (if (`self.dead?`)
    (bind _asthird_person_character (cast `/Game/Blueprints/ThirdPersonCharacter` OtherActor))
    (set `/Game/Blueprints/ThirdPersonCharacter.HighlightedZombieCorpse?` true _asthird_person_character)
    (set `/Game/Blueprints/ThirdPersonCharacter.ZombieCorpseRef` self _asthird_person_character)))

(event `RegisterInteractable`
  (`PrimitiveComponent.SetRenderCustomDepth` (`self.Mesh`) true))

(event `self.ZombieCorpseRadius.OnComponentEndOverlap`
  (params (OverlappedComponent :type "PrimitiveComponent Object Reference") (OtherActor :type "Actor Object Reference") (OtherComp :type "PrimitiveComponent Object Reference") (OtherBodyIndex :type Integer))
  (if (`self.dead?`)
    (bind _asthird_person_character (cast `/Game/Blueprints/ThirdPersonCharacter` OtherActor))
    (set `/Game/Blueprints/ThirdPersonCharacter.HighlightedZombieCorpse?` false _asthird_person_character)
    (set `/Game/Blueprints/ThirdPersonCharacter.ZombieCorpseRef` null _asthird_person_character)
    (`PrimitiveComponent.SetRenderCustomDepth` (`self.Mesh`) false :!label _label)))

(event `UnregisterInteractable`
  (goto _label))

(event `GetClosestPoint`
  ;[1 1 1] Navigation
  (bind _outactors (`GameplayStatics.GetAllActorsWithTag` "NavigationPoint"))
  (set `self.ClosestNavPoint` (`|GetArrayItem` _outactors))
  (for (_array_element _array_index) _outactors
    (if (!= _array_index 0)
      (if (< (`self.GetDistanceTo` _array_element self) (`self.GetDistanceTo` (`self.ClosestNavPoint`) self))
        (set `self.ClosestNavPoint` _array_element))))
  (set `self.NextNavPoint` (cast `/Game/Blueprints/NavigationPoint` (`self.ClosestNavPoint`) :!pure true)))

(event `self.ReceiveBeginPlay`
  (bind _players (`/Game/ThirdPerson/ThirdPersonGameMode.Players` (cast `/Game/ThirdPerson/ThirdPersonGameMode` (`GameplayStatics.GetGameMode`) :!pure true)))
  ;[1 1 1] EventBeginPlay
  (`|ExecutionSequence`
    (:`then_0`
      (set `self.ClosestPlayer` (`|GetArrayItem` _players))
      (for _array_element _players
        (if (<= (`self.GetDistanceTo` _array_element) (`self.GetDistanceTo` (`self.ClosestPlayer`)))
          (set `self.ClosestPlayer` _array_element))))
    (:`then_1`
      (`KismetSystemLibrary.Delay` 0.4)
      (`SceneComponent.SetVisibility` (`self.Mesh`) true false))))

(event `EnableNavigation`
  ;[1 1 1] Navigation
  (`AITask_MoveTo.AIMoveTo` (`AIBlueprintHelperLibrary.GetAIController` self) (0.0 0.0 0.0) (`self.ClosestPlayer`) :!label _label_2
    (:`OnMoveFinished`
      (`KismetSystemLibrary.Delay` 0.5)
      (if (not (`self.dead?`))
        (goto _label_2)))))

(event `MoveToNextPoint`
  (params (NextPoint :type "/Game/Blueprints/NavigationPoint Object Reference"))
  ;[1 1 1] Navigation
)

(event `self.ReceiveTick`
  (params (DeltaSeconds :type "Float (single-precision)"))
  (`|ExecutionSequence`
    (:`then_0`
      (if (`self.dead?`)
        _
        (elif (<= (`self.GetDistanceTo` (`self.ClosestPlayer`)) 100.0)
          (if (`self.Attack`)
            (goto _label_3 :!via `Reset`)
            (else
              (`/Engine/EditorBlueprintResources/StandardMacros.DoOnce` false :!label _label_3
                (:`Completed`
                  (set `self.Attack` true)
                  (for _array_element (`PrimitiveComponent.GetOverlappingActors` (`self.MeleeHitDetection`) "/Game/Blueprints/ThirdPersonCharacter.ThirdPersonCharacter_C")
                    (`GameplayStatics.SpawnEmitterAttached` "/Game/Art/Effects/BloodHit.BloodHit" (`Character.Mesh` (cast `/Game/Blueprints/ThirdPersonCharacter` _array_element :!pure true)) "Head" (0.0 0.0 0.0) (struct) (0.25 0.25 0.25) "SnapToTarget")
                    (`GameplayStatics.ApplyDamage` _array_element 10.0)
                    (`KismetSystemLibrary.Delay` 0.5)
                    (set `self.Attack` false)))))))))
    (:`then_1`)))

(event `self.ReceiveAnyDamage`
  (params (Damage :type "Float (single-precision)") (DamageType :type "DamageType Object Reference") (InstigatedBy :type "Controller Object Reference") (DamageCauser :type "Actor Object Reference"))
  (bind _capsulecomponent (`self.CapsuleComponent`))
  (bind _returnvalue_location (`KismetMathLibrary.BreakTransform` (`SceneComponent.K2_GetComponentToWorld` (`self.LootSpawn`))))
  ;[1 1 1] Take Damage
  (bind _output_get (set `self.Health` (- (`self.Health`) Damage)))
  (if (<= _output_get 0.0)
    ;[1 1 1] Dead
    (set `self.dead?` true :!label _label_4)
    (`KismetSystemLibrary.PrintString` "DEAD ZOMBIE")
    (`MovementComponent.StopMovementImmediately` (`self.CharacterMovement`))
    (`PrimitiveComponent.SetCollisionEnabled` (`self.CapsuleComponent`) "NoCollision")
    (`Controller.StopMovement` (`AIBlueprintHelperLibrary.GetAIController` (`self.GetController`)))
    (`PrimitiveComponent.SetCollisionResponseToChannel` _capsulecomponent "ECC_Pawn" "ECR_Ignore")
    (`PrimitiveComponent.SetCollisionResponseToChannel` _capsulecomponent "ECC_WorldDynamic" "ECR_Ignore")
    (`PrimitiveComponent.SetSimulatePhysics` (`self.Mesh`) true)
    (bind _returnvalue (`|SpawnActorFromClass` "/Game/Blueprints/WeddingRing.WeddingRing_C" (`KismetMathLibrary.MakeTransform` _returnvalue_location (`KismetMathLibrary.RandomRotator` true)) "AdjustIfPossibleButAlwaysSpawn" "OverrideRootScale" null null))
    (bind _staticmesh (`/Game/Blueprints/WeddingRing.StaticMesh` _returnvalue))
    (`PrimitiveComponent.AddImpulse` _staticmesh (0.0 0.0 500.0) "None" true)
    (`PrimitiveComponent.AddTorqueInRadians` _staticmesh (* (`KismetMathLibrary.RandomUnitVector`) 500.0) "None" true)
    (else
      ;[1 1 1] NotKillingBlow - physics on part
      (switch `int` (`KismetMathLibrary.RandomIntegerInRange` 0 3)
        (:`0`
          (`SkeletalMeshComponent.SetAllBodiesBelowSimulatePhysics` (`self.Mesh`) (`KismetStringLibrary.Conv_StringToName` "spine1") true true))
        (:`1`
          (`SkeletalMeshComponent.SetAllBodiesBelowSimulatePhysics` (`self.Mesh`) (`KismetStringLibrary.Conv_StringToName` "Neck") true true))
        (:`2`
          (`SkeletalMeshComponent.SetAllBodiesBelowSimulatePhysics` (`self.Mesh`) (`KismetStringLibrary.Conv_StringToName` "RightArm") true true))
        (:`3`
          (`SkeletalMeshComponent.SetAllBodiesBelowSimulatePhysics` (`self.Mesh`) (`KismetStringLibrary.Conv_StringToName` "LeftArm") true true))))))

(event `Kill`
  ;[1 1 1] Dead
  (goto _label_4))

(event `PickUp`
  (params (CarryingPlayerRef :type "/Game/Blueprints/ThirdPersonCharacter Object Reference"))
  (bind _mesh (`self.Mesh`))
  (bind _zombie_locked (`self.Zombie_LOCKED`))
  (bind _zombie_locked_2 (`self.Zombie_LOCKED`))
  (bind _carryingplayerref (`self.CarryingPlayerRef`))
  ;[1 1 1] Pickup
  (bind _output_get (set `self.CarryingPlayerRef` CarryingPlayerRef))
  (set `/Game/Blueprints/ThirdPersonCharacter.HoldingCorpse?` true CarryingPlayerRef)
  (`/Game/Blueprints/ThirdPersonCharacter.PickedUpCorpse` _output_get self)
  (`SceneComponent.K2_SetWorldLocation` (`self.Zombie_LOCKED`) (`SceneComponent.K2_GetComponentLocation` (`self.Mesh`)) false true)
  (`SceneComponent.SetVisibility` (`self.Mesh`) false false)
  (`SceneComponent.SetVisibility` _zombie_locked true false)
  (`PrimitiveComponent.SetCollisionEnabled` _zombie_locked "QueryAndPhysics")
  (`PrimitiveComponent.SetCollisionEnabled` (`self.Mesh`) "NoCollision")
  (set `self.StartPos` (`SceneComponent.GetSocketLocation` (`self.Mesh`) "Hips"))
  (`Timeline|Timeline_0` :!via `PlayFromStart`
    (:`Update`
      (`SceneComponent.K2_SetWorldLocation` (`self.Zombie_LOCKED`) (`KismetMathLibrary.VLerp` (`self.StartPos`) (`SceneComponent.GetSocketLocation` (`Character.Mesh` (`self.CarryingPlayerRef`)) "RightHand_ItemJoint")) false false))
    (:`Finished`
      (`self.K2_AttachToComponent` (`Character.Mesh` _carryingplayerref) "RightHand_ItemJoint" "SnapToTarget" "SnapToTarget" "SnapToTarget" false)
      (`SceneComponent.K2_SetWorldLocation` _zombie_locked_2 (`SceneComponent.GetSocketLocation` (`Character.Mesh` _carryingplayerref) "RightHand_ItemJoint") false true)
      (`SceneComponent.K2_SetWorldLocation` (`self.Mesh`) (`SceneComponent.GetSocketLocation` (`Character.Mesh` _carryingplayerref) "RightHand_ItemJoint") false true)
      (`SceneComponent.K2_SetRelativeLocationAndRotation` _zombie_locked_2 (92.263306 11.380176 19.997604) (struct :`Pitch` 1.678942 :`Yaw` -82.998062 :`Roll` -99.714676) false true)
      (`SceneComponent.K2_SetRelativeLocationAndRotation` (`self.Mesh`) (92.263306 11.380176 19.997604) (struct :`Pitch` 1.678942 :`Yaw` -82.998062 :`Roll` -99.714676) false true) ; ????
      (`PrimitiveComponent.SetCollisionEnabled` _mesh "NoCollision")
      (`PrimitiveComponent.SetSimulatePhysics` (`self.Zombie_LOCKED`) true)
      (`PrimitiveComponent.SetSimulatePhysics` _mesh false))))

(event `DropCorpse`
  (bind _carryingplayerref (`self.CarryingPlayerRef`))
  (bind _mesh (`self.Mesh`))
  (bind _zombie_locked (`self.Zombie_LOCKED`))
  (bind _zombie_locked_2 (`self.Zombie_LOCKED`))
  ;[1 1 1] Drop Corpse
  (`/Game/Blueprints/ThirdPersonCharacter.DropedCorpse` (`self.CarryingPlayerRef`))
  (`self.K2_DetachFromActor` "KeepWorld" "KeepWorld" "KeepWorld")
  (set `self.StartPos` (`self.K2_GetActorLocation`))
  (bind (_direction _newtrack_0) (`Timeline|Timeline_1` :!via `PlayFromStart`)
    (:`Update`
      (`self.K2_SetActorLocation` (`KismetMathLibrary.VLerp` (`self.StartPos`) (+ (`self.K2_GetActorLocation` _carryingplayerref) (* (`SceneComponent.GetForwardVector` (`Actor.RootComponent` _carryingplayerref)) 50.0)) _newtrack_0)))
    (:`Finished`
      (`SceneComponent.K2_SetRelativeLocationAndRotation` (`self.Mesh`) (`SceneComponent.K2_GetComponentLocation` _zombie_locked) (`SceneComponent.K2_GetComponentRotation` _zombie_locked) false false)
      (`SceneComponent.SetVisibility` (`self.Mesh`) true false)
      (`SceneComponent.SetVisibility` _zombie_locked_2 false false)
      (`PrimitiveComponent.SetCollisionEnabled` _zombie_locked_2 "NoCollision") ; 1
      (`PrimitiveComponent.SetCollisionEnabled` _mesh "QueryAndPhysics")
      (`PrimitiveComponent.SetCollisionEnabled` _mesh "QueryAndPhysics")
      (`PrimitiveComponent.SetSimulatePhysics` (`self.Zombie_LOCKED`) false) ; 1
      (`PrimitiveComponent.SetSimulatePhysics` _mesh true)
      (if (<= (`KismetMathLibrary.Vector_Distance` (`SceneComponent.K2_GetComponentLocation` (`Character.Mesh` (`self.CarryingPlayerRef`))) (`SceneComponent.K2_GetComponentLocation` (`self.Mesh`))) 180.0)
        (`self.RegisterInteractable`)
        (else
          (`self.UnregisterInteractable`)))
      (set `self.CarryingPlayerRef` null))))

(fn `UserConstructionScript`)