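; Corpse actor that a player can pick up, carry in the right hand and drop, with a random name from a data table shown on it.
; It swaps visibility, collision and physics between a free ragdoll SkeletalMesh and a LockedSkeletalMesh used while carried.
; Interaction saves a pose snapshot and, after a timeline, attaches to the hand socket.
; Dropping detaches, lerps the actor before the carrier and restores the free mesh.
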(event `self.ReceiveBeginPlay`
  (bind _lockedskeletalmesh (`self.LockedSkeletalMesh`))
  (`SceneComponent.K2_AttachToComponent` (`self.InteractableAreaaaaaa`) (`self.SkeletalMesh`) "None" "KeepRelative" "KeepRelative" "KeepRelative" true) ; attachInteractableAreaToMesh
  (`SceneComponent.SetVisibility` (`self.SkeletalMesh`) true false)
  (`SceneComponent.SetVisibility` _lockedskeletalmesh false false)
  (`PrimitiveComponent.SetCollisionEnabled` _lockedskeletalmesh "NoCollision")
  (`PrimitiveComponent.SetCollisionEnabled` (`self.SkeletalMesh`) "QueryAndPhysics")
  (`PrimitiveComponent.SetSimulatePhysics` (`self.LockedSkeletalMesh`) false)
  (`PrimitiveComponent.SetSimulatePhysics` (`self.SkeletalMesh`) true))

(event `/Game/Blueprints/InteractableInterface.InteractedFunction`
  (params (PlayerInteracted :type "/Game/Blueprints/ThirdPersonCharacter Object Reference"))
  (bind _skeletalmesh (`self.SkeletalMesh`))
  (bind _skeletalmesh_2 (`self.SkeletalMesh`))
  (bind _carryingplayerref (`self.CarryingPlayerRef`))
  (bind _lockedskeletalmesh (`self.LockedSkeletalMesh`))
  ;[1 1 1] Interacted Event
  (set `self.CarryingPlayerRef` PlayerInteracted)
  (set `/Game/Blueprints/ThirdPersonCharacter.HoldingCorpse?` true PlayerInteracted)
  (set `self.IsCarried?` true)
  (`/Game/Blueprints/ThirdPersonCharacter.PickedUpCorpse` PlayerInteracted self)
  (`SceneComponent.K2_SetWorldLocation` (`self.LockedSkeletalMesh`) (`SceneComponent.K2_GetComponentLocation` _skeletalmesh) false true)
  (`AnimInstance.SavePoseSnapshot` (`SkeletalMeshComponent.GetAnimInstance` _skeletalmesh) "GroundPose")
  (`SceneComponent.SetVisibility` (`self.SkeletalMesh`) false false)
  (`SceneComponent.SetVisibility` _lockedskeletalmesh true false)
  (`PrimitiveComponent.SetCollisionEnabled` _lockedskeletalmesh "QueryAndPhysics")
  (`PrimitiveComponent.SetCollisionEnabled` (`self.SkeletalMesh`) "NoCollision")
  (set `self.StartPos` (`SceneComponent.K2_GetComponentLocation` (`self.LockedSkeletalMesh`)))
  (`Timeline|Timeline_1` :!via `PlayFromStart`
    (:`Update`
      (`SceneComponent.K2_SetWorldLocation` (`self.LockedSkeletalMesh`) (`KismetMathLibrary.VLerp` (`self.StartPos`) (`SceneComponent.GetSocketLocation` (`Character.Mesh` (`self.CarryingPlayerRef`)) "RightHand_ItemJoint")) false false))
    (:`Finished`
      (`self.K2_AttachToComponent` (`Character.Mesh` _carryingplayerref) "RightHand_ItemJoint" "SnapToTarget" "SnapToTarget" "SnapToTarget" false)
      (`SceneComponent.K2_SetWorldLocation` _skeletalmesh_2 (`SceneComponent.GetSocketLocation` (`Character.Mesh` _carryingplayerref) "RightHand_ItemJoint") false true)
      (`SceneComponent.K2_SetWorldLocation` (`self.LockedSkeletalMesh`) (`SceneComponent.GetSocketLocation` (`Character.Mesh` _carryingplayerref) "RightHand_ItemJoint") false true)
      (`SceneComponent.K2_SetRelativeLocationAndRotation` _skeletalmesh_2 (0.0 0.0 0.0) (struct :`Yaw` 90.0 :`Roll` 180.0) false true)
      (`SceneComponent.K2_SetRelativeLocationAndRotation` (`self.LockedSkeletalMesh`) (0.0 0.0 0.0) (struct :`Yaw` 90.0 :`Roll` 180.0) false true) ; ????
      (`PrimitiveComponent.SetCollisionEnabled` (`self.SkeletalMesh`) "NoCollision")
      (`PrimitiveComponent.SetSimulatePhysics` (`self.LockedSkeletalMesh`) true)
      (`PrimitiveComponent.SetSimulatePhysics` (`self.SkeletalMesh`) false))))

(event `DropedCorpse`
  (bind _carryingplayerref (`self.CarryingPlayerRef`))
  (bind _skeletalmesh (`self.SkeletalMesh`))
  (bind _lockedskeletalmesh (`self.LockedSkeletalMesh`))
  (bind _lockedskeletalmesh_2 (`self.LockedSkeletalMesh`))
  ;[1 1 1] Drop Corpse
  (set `self.IsCarried?` false)
  (`/Game/Blueprints/ThirdPersonCharacter.DropedCorpse` (`self.CarryingPlayerRef`))
  (`/Engine/EditorBlueprintResources/StandardMacros.IsValid` self
    (:`Is Valid`
      (`self.K2_DetachFromActor` "KeepWorld" "KeepWorld" "KeepWorld")
      (set `self.StartPos` (`self.K2_GetActorLocation`))
      (bind (_direction _newtrack_0) (`Timeline|Timeline_0` :!via `PlayFromStart`)
        (:`Update`
          (`self.K2_SetActorLocation` (`KismetMathLibrary.VLerp` (`self.StartPos`) (+ (`self.K2_GetActorLocation` _carryingplayerref) (* (`SceneComponent.GetForwardVector` (`Actor.RootComponent` _carryingplayerref)) 50.0)) _newtrack_0)))
        (:`Finished`
          (`SceneComponent.K2_SetRelativeLocationAndRotation` (`self.SkeletalMesh`) (`SceneComponent.K2_GetComponentLocation` _lockedskeletalmesh) (`SceneComponent.K2_GetComponentRotation` _lockedskeletalmesh) false false)
          (`SceneComponent.SetVisibility` (`self.SkeletalMesh`) true false)
          (`SceneComponent.SetVisibility` _lockedskeletalmesh_2 false false)
          (`PrimitiveComponent.SetCollisionEnabled` _lockedskeletalmesh_2 "NoCollision") ; 1
          (`PrimitiveComponent.SetCollisionEnabled` _skeletalmesh "QueryAndPhysics")
          (`PrimitiveComponent.SetCollisionEnabled` _skeletalmesh "QueryAndPhysics")
          (`PrimitiveComponent.SetSimulatePhysics` (`self.LockedSkeletalMesh`) false) ; 1
          (`PrimitiveComponent.SetSimulatePhysics` _skeletalmesh true)
          (set `self.CarryingPlayerRef` null))))))

(fn `UserConstructionScript`
  (bind _returnvalue (`DataTableFunctionLibrary.GetDataTableColumnAsString` "/Game/Blueprints/ListOfNames.ListOfNames" "Name"))
  (bind _output_get (set `self.CorpseName` (`KismetStringLibrary.Conv_StringToName` (`|GetArrayItem` _returnvalue (`KismetMathLibrary.RandomIntegerInRange` 0 (- (`KismetArrayLibrary.Array_Length` _returnvalue) 1))))))
  (`TextRenderComponent.K2_SetText` (`self.Name`) (`KismetTextLibrary.Conv_NameToText` _output_get)))