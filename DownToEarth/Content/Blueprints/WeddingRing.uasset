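; Wedding ring pickup that becomes collectable shortly after spawn and counts as currency for all players.
; On overlap with a ThirdPersonCharacter, it disables mesh physics and collision, then runs timelines that scale the mesh and move it toward that player.
; A Tick gate keeps updating the target to just above the player's location.
; When movement finishes, it calls CollectedCurrency on every player in the game mode and destroys itself.
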(event `self.ReceiveBeginPlay`
  (`KismetSystemLibrary.Delay` 0.3)
  (set `self.Collectable?` true))

(event `self.CollectionArea.OnComponentBeginOverlap`
  (params (OverlappedComponent :type "PrimitiveComponent Object Reference") (OtherActor :type "Actor Object Reference") (OtherComp :type "PrimitiveComponent Object Reference") (OtherBodyIndex :type Integer) (bFromSweep :type Boolean) (SweepResult :type "HitResult Structure (by ref)"))
  (bind _staticmesh (`self.StaticMesh`))
  (if (`self.Collectable?`)
    (if (== (`GameplayStatics.GetObjectClass` OtherActor) "/Game/Blueprints/ThirdPersonCharacter.ThirdPersonCharacter_C")
      (set `self.PlayerReference` OtherActor)
      (`PrimitiveComponent.SetSimulatePhysics` _staticmesh false)
      (`PrimitiveComponent.SetCollisionEnabled` _staticmesh "NoCollision")
      (`|ExecutionSequence`
        (:`then_0`
          (`/Engine/EditorBlueprintResources/StandardMacros.DoOnce` false
            (:`Completed`
              (set `self.StartLoc` (`SceneComponent.K2_GetComponentLocation` (`self.StaticMesh`)))
              (`|ExecutionSequence`
                (:`then_0`
                  (bind (_direction _newtrack_0) (`Timeline|Timeline_1` :!via `PlayFromStart`)
                    (:`Update`
                      (`SceneComponent.SetRelativeScale3D` (`self.StaticMesh`) (`KismetMathLibrary.VLerp` (0.0 0.0 0.0) (1.0 1.0 1.0) _newtrack_0)))))
                (:`then_1`
                  (bind (_direction_2 _newtrack_0_2) (`Timeline|Timeline_0` :!via `PlayFromStart`)
                    (:`Update`
                      (`SceneComponent.K2_SetWorldLocation` (`self.StaticMesh`) (`KismetMathLibrary.VLerp` (`self.StartLoc`) (`self.EndPos`) _newtrack_0_2) false false))
                    (:`Finished`
                      (`self.Collected`)
                      (for _array_element (`/Game/ThirdPerson/ThirdPersonGameMode.Players` (cast `/Game/ThirdPerson/ThirdPersonGameMode` (`GameplayStatics.GetGameMode`) :!pure true))
                        (`/Game/Blueprints/ThirdPersonCharacter.Collected Currency` _array_element))
                      (`self.K2_DestroyActor`))))))))
        (:`then_1`
          (goto _label :!via `Open`))))))

(event `self.ReceiveTick`
  (params (DeltaSeconds :type "Float (single-precision)"))
  (`/Engine/EditorBlueprintResources/StandardMacros.Gate` true :!label _label
    (:`Exit`
      (set `self.EndPos` (+ (`self.K2_GetActorLocation` (`self.PlayerReference`)) (0.0 0.0 50.0))))))

(event `Collected`
  (goto _label :!via `Close`))

(fn `UserConstructionScript`)