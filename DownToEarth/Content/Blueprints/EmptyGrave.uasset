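; Empty grave actor that absorbs a dropped corpse and, once filled, spawns a zombie once when night initiates.
; An uncarried Corpse entering or leaving its box triggers FillGrave, which records name and type, swaps plot for mound, plays dust and clears the carrier's reference.
; A detection volume highlights unfilled graves for corpse-carrying players through a dynamic dirt material and point light.
; The old interact event only prints debug messages.
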(event `/Game/Blueprints/InteractableInterface.InteractedFunction`
  (params (PlayerInteracted :type "/Game/Blueprints/ThirdPersonCharacter Object Reference"))
  ;[1 1 1] Old Interact on grave
  (if (`self.IsFilled?`)
    (`KismetSystemLibrary.PrintString` "Grave is already Full" :!label _label)
    (elif (not (`/Game/Blueprints/ThirdPersonCharacter.HoldingCorpse?` PlayerInteracted))
      (`KismetSystemLibrary.PrintString` "Not Holding Corpse"))))

(event `FillGrave`
  (params (Corpse :type "/Game/Blueprints/Corpse Object Reference"))
  (bind _carryingplayerref (`/Game/Blueprints/Corpse.CarryingPlayerRef` Corpse))
  (if (`self.IsFilled?`)
    (goto _label)
    (elif (not (`/Game/Blueprints/Corpse.AbsorbedIntoOneGrave?` Corpse))
      (set `self.IsFilled?` true)
      (`|ExecutionSequence`
        (:`then_0`
          ;[1 1 1] Set GraveName
          (bind _output_get (set `self.DeadName` (`KismetTextLibrary.Conv_NameToText` (`/Game/Blueprints/Corpse.CorpseName` Corpse))))
          (set `self.HoldingCorpseType` (`/Game/Blueprints/Corpse.CorpseType` Corpse))
          (`TextRenderComponent.K2_SetText` (`/Game/Blueprints/Corpse.Name` Corpse) _output_get)
          (`KismetSystemLibrary.PrintString` (`KismetStringLibrary.Concat_StrStr` "Grave is now Filled with " (`KismetTextLibrary.Conv_TextToString` (`self.DeadName`))))
          (`TextRenderComponent.K2_SetText` (`self.CorpseTypeText`) (`KismetTextLibrary.Conv_StringToText` (`|GetEnumeratorNameAsString` (`self.HoldingCorpseType`)))))
        (:`then_1`
          ;[1 1 1] Change GravePlot Model
          (`SceneComponent.SetVisibility` (`self.DirtPlot01`) false false)
          (`SceneComponent.SetVisibility` (`self.DirtMound01`) true false)
          (`SceneComponent.SetVisibility` (`self.NameOfDead`) true false)
          (`ActorComponent.Activate` (`self.Dust`) false)
          (`SceneComponent.SetVisibility` (`self.PointLight`) false false))
        (:`then_2`
          ;[1 1 1] Destroy Filled Grave zombioe
          (`/Engine/EditorBlueprintResources/StandardMacros.IsValid` _carryingplayerref
            (:`Is Valid`
              (set `/Game/Blueprints/ThirdPersonCharacter.CarriedCorpse` null _carryingplayerref)
              (set `/Game/Blueprints/ThirdPersonCharacter.HoldingCorpse?` false _carryingplayerref))
            (:`Is Not Valid`
              _))
          (`/Game/Blueprints/Corpse.Filled Grave` Corpse))))))

(event `NightTimeInitate`
  (bind (_returnvalue_location _returnvalue_rotation) (`KismetMathLibrary.BreakTransform` (`SceneComponent.K2_GetComponentToWorld` (`self.SpawnPosition`))))
  ;[1 1 1] SpawnZombies
  (if (and (not (`self.HasSpawnedZombie`)) (`self.IsFilled?`))
    (`AIBlueprintHelperLibrary.SpawnAIFromClass` "/Game/Blueprints/Zombie_Base.Zombie_Base_C" null _returnvalue_location _returnvalue_rotation)
    (set `self.HasSpawnedZombie` true)))

(event `self.Box.OnComponentBeginOverlap`
  (params (OverlappedComponent :type "PrimitiveComponent Object Reference") (OtherActor :type "Actor Object Reference") (OtherComp :type "PrimitiveComponent Object Reference") (OtherBodyIndex :type Integer) (bFromSweep :type Boolean) (SweepResult :type "HitResult Structure (by ref)"))
  ;[1 1 1] Absorb Zombies
  (if (== (`GameplayStatics.GetObjectClass` OtherActor) "/Game/Blueprints/Corpse.Corpse_C")
    (bind _ascorpse (cast `/Game/Blueprints/Corpse` OtherActor))
    (if (not (`/Game/Blueprints/Corpse.IsCarried?` _ascorpse))
      (`self.FillGrave` _ascorpse))))

(event `self.ReceiveTick`
  (params (DeltaSeconds :type "Float (single-precision)"))
  (bind _isfilled_ (`self.IsFilled?`))
  (if (`self.GraveHighlighted`)
    (if (not _isfilled_)
      (goto _label_2 :!via `Reset`))
    (elif (not _isfilled_)
      (`/Engine/EditorBlueprintResources/StandardMacros.DoOnce` false :!label _label_2
        (:`Completed`
          (`MaterialInstanceDynamic.SetScalarParameterValue` (`self.InstancedMaterial`) "EmissiveStrength" 0.0)
          (`SceneComponent.SetVisibility` (`self.PointLight`) false false))))))

(event `self.Box.OnComponentEndOverlap`
  (params (OverlappedComponent :type "PrimitiveComponent Object Reference") (OtherActor :type "Actor Object Reference") (OtherComp :type "PrimitiveComponent Object Reference") (OtherBodyIndex :type Integer))
  ;[1 1 1] Absorb Zombies
  (if (== (`GameplayStatics.GetObjectClass` OtherActor) "/Game/Blueprints/Corpse.Corpse_C")
    (bind _ascorpse (cast `/Game/Blueprints/Corpse` OtherActor))
    (if (not (`/Game/Blueprints/Corpse.IsCarried?` _ascorpse))
      (`self.FillGrave` _ascorpse))))

(event `self.ActorDetect.OnComponentBeginOverlap`
  (params (OverlappedComponent :type "PrimitiveComponent Object Reference") (OtherActor :type "Actor Object Reference") (OtherComp :type "PrimitiveComponent Object Reference") (OtherBodyIndex :type Integer) (bFromSweep :type Boolean) (SweepResult :type "HitResult Structure (by ref)"))
  (if (`self.IsFilled?`)
    _
    (elif (== (`GameplayStatics.GetObjectClass` OtherActor) "/Game/Blueprints/ThirdPersonCharacter.ThirdPersonCharacter_C")
      (bind _asthird_person_character (cast `/Game/Blueprints/ThirdPersonCharacter` OtherActor))
      (`/Engine/EditorBlueprintResources/StandardMacros.IsValid` _asthird_person_character
        (:`Is Valid`
          (if (`/Game/Blueprints/ThirdPersonCharacter.HoldingCorpse?` _asthird_person_character)
            (set `self.GraveHighlighted` true)
            (`MaterialInstanceDynamic.SetScalarParameterValue` (`self.InstancedMaterial`) "EmissiveStrength" 2.0)
            (`SceneComponent.SetVisibility` (`self.PointLight`) true false)
            (else
              (set `self.GraveHighlighted` false :!label _label_3)
              (`MaterialInstanceDynamic.SetScalarParameterValue` (`self.InstancedMaterial`) "EmissiveStrength" 0.0)
              (`SceneComponent.SetVisibility` (`self.PointLight`) false false))))))))

(event `self.ActorDetect.OnComponentEndOverlap`
  (params (OverlappedComponent :type "PrimitiveComponent Object Reference") (OtherActor :type "Actor Object Reference") (OtherComp :type "PrimitiveComponent Object Reference") (OtherBodyIndex :type Integer))
  (if (`self.IsFilled?`)
    _
    (elif (== (`GameplayStatics.GetObjectClass` OtherActor) "/Game/Blueprints/ThirdPersonCharacter.ThirdPersonCharacter_C")
      (goto _label_3)
      (else
        (for _array_element (`PrimitiveComponent.GetOverlappingActors` (`self.ActorDetect`) null)
          (if (== (`GameplayStatics.GetObjectClass` _array_element) "/Game/Blueprints/Zombie_Base.Zombie_Base_C")
            (break)))
        (goto _label_3)))))

(fn `UserConstructionScript`
  (bind _returnvalue (`PrimitiveComponent.CreateDynamicMaterialInstance` (`self.DirtPlot01`) 0 "/Game/Art/Objects/TombStone/dirt_plot_Inst.dirt_plot_Inst" "None"))
  (set `self.InstancedMaterial` _returnvalue))