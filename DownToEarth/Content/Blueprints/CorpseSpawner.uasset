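; Corpse chute actor that spawns one Corpse per EmptyGrave in the level and pushes corpses along a conveyor.
; BeginPlay counts the graves, then Tick drives a Delay-gated spawn at CorpseSpawnPoint until that count runs out.
; Each tick also applies an impulse along the Arrow's forward vector to every bone of tagged skeletal meshes on corpses overlapping ConveyorForce.
; Belt material, ragdoll, timeline and unclaimed-corpse check logic is left disconnected.
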(event `SpawnNewCorpse`
  (`|SpawnActorFromClass` "/Game/Blueprints/Corpse.Corpse_C" (`SceneComponent.K2_GetComponentToWorld` (`self.CorpseSpawnPoint`)) "Undefined" "OverrideRootScale" null null))

(event `self.ReceiveBeginPlay`
  (bind _outactors (`GameplayStatics.GetAllActorsOfClass` "/Game/Blueprints/EmptyGrave.EmptyGrave_C"))
  (set `self.NumberOfCorpses` (`KismetArrayLibrary.Array_Length` _outactors)))

(event `SpawnCorpses`
  (if (> (`self.NumberOfCorpses`) 0)
    (`KismetSystemLibrary.Delay` (`self.SpawnFrequency`))
    (`self.SpawnNewCorpse`)
    (set `self.NumberOfCorpses` (- (`self.NumberOfCorpses`) 1))))

(event `self.ReceiveTick`
  (params (DeltaSeconds :type "Float (single-precision)"))
  (`|ExecutionSequence`
    (:`then_0`
      (`self.SpawnCorpses`))
    (:`then_1`
      (`self.MoveActorsAlongConveyor`))))

(event `MoveActorsAlongConveyor`
  (for _array_element (`PrimitiveComponent.GetOverlappingActors` (`self.conveyor_force`) "/Game/Blueprints/Corpse.Corpse_C")
    (for _array_element_2 (`self.GetComponentsByTag` _array_element "/Script/Engine.ActorComponent" "skelMesh")
      ;[1 0 0] CASTING EVERY TICK IS NOT AWESOME!
      (bind _asskeletal_mesh_component (cast `SkeletalMeshComponent` _array_element_2))
      (for _index (range (`SkinnedMeshComponent.GetNumBones` _asskeletal_mesh_component))
        (bind _returnvalue (`SkinnedMeshComponent.GetBoneName` _asskeletal_mesh_component _index))
        (`PrimitiveComponent.AddImpulseAtLocation` _asskeletal_mesh_component (* (`SceneComponent.GetForwardVector` (`self.Arrow`)) (`self.Speed`)) (`SceneComponent.GetSocketLocation` _asskeletal_mesh_component _returnvalue) _returnvalue)))))

(fn `UserConstructionScript`)