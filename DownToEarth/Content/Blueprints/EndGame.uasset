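; EndGame is a trigger that ends the game when the player character enters its Box component.
; On overlap it checks for the ThirdPersonCharacter class and ignores that character's MeleeHitDetection component.
; It then shows the WINSCREEN widget to player controller 0 and loads the MainMenu level after a delay.
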(event `self.Box.OnComponentBeginOverlap`
  (params (OverlappedComponent :type "PrimitiveComponent Object Reference") (OtherActor :type "Actor Object Reference") (OtherComp :type "PrimitiveComponent Object Reference") (OtherBodyIndex :type Integer) (bFromSweep :type Boolean) (SweepResult :type "HitResult Structure (by ref)"))
  (if (== (`GameplayStatics.GetObjectClass` OtherActor) "/Game/Blueprints/ThirdPersonCharacter.ThirdPersonCharacter_C")
    (bind _asthird_person_character (cast `/Game/Blueprints/ThirdPersonCharacter` OtherActor))
    (if (!= OtherComp (`/Game/Blueprints/ThirdPersonCharacter.MeleeHitDetection` _asthird_person_character))
      (bind _returnvalue (`|CreateWidget` "/Game/HUD/WINSCREEN.WINSCREEN_C" (`GameplayStatics.GetPlayerController` 0))) ; NotUsedWhenOnSharedCamer
      (`UserWidget.AddToViewport` _returnvalue 0)
      (`KismetSystemLibrary.Delay` 10.0)
      (`GameplayStatics.OpenLevel` "MainMenu"))))

(fn `UserConstructionScript`)