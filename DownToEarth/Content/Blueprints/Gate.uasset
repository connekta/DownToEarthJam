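; Interactable double gate that swings open once when interacted with, unless it is locked.
; Overlapping the interactable area toggles custom depth on both leaves as a highlight while the gate is unlocked and closed.
; Interaction sets Open, clears the highlight and plays the GateOpen timeline, rotating the leaves in opposite yaw directions up to RotationSpeed, which acts as the final angle.
; No closing logic exists, and leftover timer nodes never run.
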(event `self.ReceiveTick`
  (params (DeltaSeconds :type "Float (single-precision)"))
  (if (`self.Open?`)
    _))

(event `/Game/Blueprints/InteractableInterface.InteractedFunction`
  (params (PlayerInteracted :type "/Game/Blueprints/ThirdPersonCharacter Object Reference"))
  (bind _rotationspeed (`self.RotationSpeed`))
  (if (`self.Locked?`)
    _
    (elif (not (`self.Open?`))
      (set `self.Open?` true)
      (`PrimitiveComponent.SetRenderCustomDepth` (`self.fencewall01_gate01`) false)
      (`PrimitiveComponent.SetRenderCustomDepth` (`self.fencewall01_gate02`) false)
      (bind (_direction _lerp) (`Timeline|GateOpen` :`NewTime` 0.0 :!via `PlayFromStart`)
        (:`Update`
          (`SceneComponent.K2_SetRelativeRotation` (`self.fencewall01_gate01`) (`KismetMathLibrary.MakeRotator` 0.0 0.0 (`KismetMathLibrary.Lerp` 0.0 _rotationspeed _lerp)) false false)
          (`SceneComponent.K2_SetRelativeRotation` (`self.fencewall01_gate02`) (`KismetMathLibrary.MakeRotator` 0.0 0.0 (`KismetMathLibrary.Lerp` 0.0 (- 0.0 _rotationspeed) _lerp)) false false)
          (if (>= 0.0 90.0)
            _))))))

(event `self.InteractableArea.OnComponentBeginOverlap`
  (params (OverlappedComponent :type "PrimitiveComponent Object Reference") (OtherActor :type "Actor Object Reference") (OtherComp :type "PrimitiveComponent Object Reference") (OtherBodyIndex :type Integer) (bFromSweep :type Boolean) (SweepResult :type "HitResult Structure (by ref)"))
  (if (`self.Locked?`)
    _
    (elif (not (`self.Open?`))
      (`PrimitiveComponent.SetRenderCustomDepth` (`self.fencewall01_gate01`) true)
      (`PrimitiveComponent.SetRenderCustomDepth` (`self.fencewall01_gate02`) true))))

(event `self.InteractableArea.OnComponentEndOverlap`
  (params (OverlappedComponent :type "PrimitiveComponent Object Reference") (OtherActor :type "Actor Object Reference") (OtherComp :type "PrimitiveComponent Object Reference") (OtherBodyIndex :type Integer))
  (if (not (`self.Locked?`))
    (`PrimitiveComponent.SetRenderCustomDepth` (`self.fencewall01_gate01`) false)
    (`PrimitiveComponent.SetRenderCustomDepth` (`self.fencewall01_gate02`) false)))

(fn `UserConstructionScript`)