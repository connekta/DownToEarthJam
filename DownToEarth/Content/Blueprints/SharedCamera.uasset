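; Shared camera actor for multiplayer games that becomes every controller's view target, frames all one to four players and creates the clock and shared HUD widgets.
; A looping timer eases it toward the players' average position, setting spring arm length from their greatest pairwise distance, clamped.
; In two-player games, when one player is left, a delayed timeline swipes to the survivor, then a gate hands over to fixed-zoom solo follow.
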(event `self.ReceiveBeginPlay`
  (if (not (== (`/Game/ThirdPerson/ThirdPersonGameMode.MaxPlayerCount` (cast `/Game/ThirdPerson/ThirdPersonGameMode` (`GameplayStatics.GetGameMode`) :!pure true)) 1))
    (`KismetSystemLibrary.Delay` 0.1)
    (`self.ClassSetup`)
    (`KismetSystemLibrary.K2_SetTimer` null "CameraUpdate" 0.001 true)
    (bind _returnvalue (`|CreateWidget` "/Game/HUD/Clock.Clock_C" (`GameplayStatics.GetPlayerController` 0)))
    (`UserWidget.AddToViewport` _returnvalue 0)
    (bind _returnvalue_2 (`|CreateWidget` "/Game/HUD/SoloPlayerHud.SoloPlayerHud_C" (`GameplayStatics.GetPlayerController` 0)))
    (bind _output_get (set `self.SoloPlayerHud` _returnvalue_2))
    (`UserWidget.AddToViewport` _output_get 0)
    (bind _outactors (`GameplayStatics.GetAllActorsOfClass` "/Game/Blueprints/ThirdPersonCharacter.ThirdPersonCharacter_C"))
    (for _array_element _outactors
      (set `/Game/Blueprints/ThirdPersonCharacter.SoloPlayerHUD` (`self.SoloPlayerHud`) _array_element))))

(event `CameraUpdate`
  (`|ExecutionSequence`
    (:`then_0`
      (switch `int` (`KismetArrayLibrary.Array_Length` (`self.PlayersArray`))
        (:`1`
          (`self.SetArmLenghtP1` :!label _label)
          (`self.SetCameraPosP1`))
        (:`2`
          (if (`self.OneManLeft?`)
            (`|ExecutionSequence`
              (:`then_0`
                (`KismetSystemLibrary.Delay` 1.0)
                (set `self.LastArmLength` (`SpringArmComponent.TargetArmLength` (`self.SpringArm`)))
                (set `self.SwipePrevPos` (`self.K2_GetActorLocation`))
                (`/Engine/EditorBlueprintResources/StandardMacros.DoOnce` false :!label _label_2
                  (:`Completed`
                    (set `self.DoneSoloSwipe` true)
                    (bind (_direction _newtrack_0) (`Timeline|Timeline_0` :!via `PlayFromStart`)
                      (:`Update`
                        (`self.K2_SetActorLocation` (`KismetMathLibrary.VLerp` (`self.SwipePrevPos`) (`self.SwipeCurrentPos`) _newtrack_0))
                        (set `SpringArmComponent.TargetArmLength` (`KismetMathLibrary.Lerp` (`self.LastArmLength`) (`self.SoloArmLength`) _newtrack_0) (`self.SpringArm`)))
                      (:`Finished`
                        (set `self.DoneSoloSwipe_02` true)
                        (goto _label_3 :!via `Open`))))))
              (:`then_1`
                (`/Engine/EditorBlueprintResources/StandardMacros.Gate` true :!label _label_3
                  (:`Exit`
                    (goto _label))))
              (:`then_2`
                (if (not (`self.DoneSoloSwipe`))
                  (`self.SetArmLenghtP2` :!label _label_4)
                  (`self.SetCameraPosP2`))))
            (else
              (`|ExecutionSequence`
                (:`then_0`
                  (goto _label_4))
                (:`then_1`
                  (`|ExecutionSequence`
                    (:`then_0`
                      (goto _label_2 :!via `Reset`))
                    (:`then_1`
                      (set `self.DoneSoloSwipe` false)
                      (set `self.DoneSoloSwipe_02` false)
                      (goto _label_3 :!via `Close`))))))))
        (:`3`
          (`self.SetArmLenghtP3`)
          (`self.SetCameraPosP3`))
        (:`4`
          (`self.SetArmLenghtP4`)
          (`self.SetCameraPosP4`))))
    (:`then_1`
      (if (and (`self.OneManLeft?`) (not (`self.DoneSoloSwipe_02`)))
        (`self.GetLastLivingPos`)))))

(fn `ClassSetup`
  (bind _asthird_person_game_mode (cast `/Game/ThirdPerson/ThirdPersonGameMode` (`GameplayStatics.GetGameMode`)))
  (bind _output_get (set `self.GameModeRef` _asthird_person_game_mode))
  (set `self.PlayersArray` (`/Game/ThirdPerson/ThirdPersonGameMode.Players` _output_get))
  (bind _outactors (`GameplayStatics.GetAllActorsOfClass` "/Script/Engine.PlayerController"))
  (`PlayerController.SetViewTargetWithBlend` _outactors self 0.0 "VTBlend_Linear" 0.0 false)
  (for (_array_element _array_index) (`self.PlayersArray`)
    (switch `int` _array_index
      (:`0`
        (set `self.P1` _array_element))
      (:`1`
        (set `self.P2` _array_element))
      (:`2`
        (set `self.P3` _array_element))
      (:`3`
        (set `self.P4` _array_element)))))

(fn `GetLastLivingPos`
  (bind _p2 (`self.P2`))
  (bind _p1 (`self.P1`))
  (if (`/Game/Blueprints/ThirdPersonCharacter.dead?` _p1)
    (set `self.SwipeCurrentPos` (`self.K2_GetActorLocation` _p2))
    (elif (`/Game/Blueprints/ThirdPersonCharacter.dead?` _p2)
      (set `self.SwipeCurrentPos` (`self.K2_GetActorLocation` _p1)))))

(fn `SetArmLenghtP1`
  (set `SpringArmComponent.TargetArmLength` (`self.SoloArmLength`) (`self.SpringArm`)))

(fn `SetArmLenghtP2`
  (set `SpringArmComponent.TargetArmLength` (`KismetMathLibrary.FClamp` (`self.GetDistanceTo` (`self.P1`) (`self.P2`)) (`self.MinArmLength`) (`self.MaxArmLength`)) (`self.SpringArm`)))

(fn `SetArmLenghtP3`
  (bind _p1 (`self.P1`))
  (bind _p2 (`self.P2`))
  (bind _p3 (`self.P3`))
  (set `SpringArmComponent.TargetArmLength` (`KismetMathLibrary.FClamp` (`.MaxValue` (`KismetMathLibrary.MaxOfFloatArray` (`|MakeArray` (`self.GetDistanceTo` _p1 _p2) (`self.GetDistanceTo` _p2 _p3) (`self.GetDistanceTo` _p1 _p3)))) (`self.MinArmLength`) (`self.MaxArmLength`)) (`self.SpringArm`)))

(fn `SetArmLenghtP4`
  (bind _p1 (`self.P1`))
  (bind _p2 (`self.P2`))
  (bind _p3 (`self.P3`))
  (bind _p4 (`self.P4`))
  (set `SpringArmComponent.TargetArmLength` (`KismetMathLibrary.FClamp` (`.MaxValue` (`KismetMathLibrary.MaxOfFloatArray` (`|MakeArray` (`self.GetDistanceTo` _p1 _p2) (`self.GetDistanceTo` _p2 _p3) (`self.GetDistanceTo` _p2 _p4) (`self.GetDistanceTo` _p1 _p3) (`self.GetDistanceTo` _p1 _p4) (`self.GetDistanceTo` _p3 _p4)))) (`self.MinArmLength`) (`self.MaxArmLength`)) (`self.SpringArm`)))

(fn `SetCameraPosP1`
  (bind _p2 (`self.P2`))
  (bind _p1 (`self.P1`))
  (if (`/Game/Blueprints/ThirdPersonCharacter.dead?` _p1)
    (set `self.CurrentPos` (`self.K2_GetActorLocation` _p2))
    (`self.K2_SetActorLocation` (`KismetMathLibrary.VInterpTo` (`self.PreviousPos`) (`self.CurrentPos`) (`GameplayStatics.GetWorldDeltaSeconds`) (`self.InterpSpeed`)) :!label _label)
    (set `self.PreviousPos` (`self.K2_GetActorLocation`))
    (elif (`/Game/Blueprints/ThirdPersonCharacter.dead?` _p2)
      (set `self.CurrentPos` (`self.K2_GetActorLocation` _p1))
      (goto _label))))

(fn `SetCameraPosP2`
  (set `self.CurrentPos` (/ (+ (`self.K2_GetActorLocation` (`self.P1`)) (`self.K2_GetActorLocation` (`self.P2`))) (`KismetMathLibrary.Conv_IntToDouble` (`KismetArrayLibrary.Array_Length` (`self.PlayersArray`)))))
  (`self.K2_SetActorLocation` (`KismetMathLibrary.VInterpTo` (`self.PreviousPos`) (`self.CurrentPos`) (`GameplayStatics.GetWorldDeltaSeconds`) (`self.InterpSpeed`)))
  (set `self.PreviousPos` (`self.K2_GetActorLocation`)))

(fn `SetCameraPosP3`
  (set `self.CurrentPos` (/ (+ (`self.K2_GetActorLocation` (`self.P1`)) (`self.K2_GetActorLocation` (`self.P2`)) (`self.K2_GetActorLocation` (`self.P3`))) (`KismetMathLibrary.Conv_IntToDouble` (`KismetArrayLibrary.Array_Length` (`self.PlayersArray`)))))
  (`self.K2_SetActorLocation` (`KismetMathLibrary.VInterpTo` (`self.PreviousPos`) (`self.CurrentPos`) (`GameplayStatics.GetWorldDeltaSeconds`) (`self.InterpSpeed`)))
  (set `self.PreviousPos` (`self.K2_GetActorLocation`)))

(fn `SetCameraPosP4`
  (set `self.CurrentPos` (/ (+ (`self.K2_GetActorLocation` (`self.P1`)) (`self.K2_GetActorLocation` (`self.P2`)) (`self.K2_GetActorLocation` (`self.P3`)) (`self.K2_GetActorLocation` (`self.P4`))) (`KismetMathLibrary.Conv_IntToDouble` (`KismetArrayLibrary.Array_Length` (`self.PlayersArray`)))))
  (`self.K2_SetActorLocation` (`KismetMathLibrary.VInterpTo` (`self.PreviousPos`) (`self.CurrentPos`) (`GameplayStatics.GetWorldDeltaSeconds`) (`self.InterpSpeed`)))
  (set `self.PreviousPos` (`self.K2_GetActorLocation`)))

(fn `UserConstructionScript`)